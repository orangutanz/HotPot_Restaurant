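; BP_Customer_AI is the customer AI controller, which runs the BT_Customer behavior tree and handles seating in the restaurant.
; FindEmptySeat gets an empty seat from the RestaurantManager, assigns it to the owning customer and marks it occupied.
; GoToSeat issues a move toward that seat, returning false until the customer is within range, then snaps it onto the seat transform.
; ChangeState stores the current state and mirrors it to a blackboard enum key.
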(event `self.ReceiveBeginPlay`
  ;[1 1 1] Get RefOf RestaurantManager
  (bind _returnvalue (`GameplayStatics.GetActorOfClass` "/Script/AI_Playground.RestaurantManager"))
  (set `self.Manager` _returnvalue)
  (`self.RunBehaviorTree` "/Game/Characters/Customer/AI/BT_Customer.BT_Customer")
  (`self.UpdateBlackboard`))

(fn `Change State`
  (params (NewState :type "/Game/Characters/Customer/AI/Enum_CustomerStates Enum" :default "NewEnumerator0"))
  (set `self.CurrentState` NewState)
  (`self.UpdateBlackboard`))

(fn `FindEmptySeat`
  (returns (FoundSeat :type Boolean))
  (bind _manager (`self.Manager`))
  ;[1 1 1] Get Valid EmptySeat
  (if (`KismetSystemLibrary.IsValid` _manager)
    (bind _returnvalue (`RestaurantManager.GetEmptySeat` _manager))
    ;[1 1 1] Found emptySeat set Occupied
    (if (`KismetSystemLibrary.IsValid` _returnvalue)
      (bind _output_get (set `/Game/Characters/Customer/BP_Customer.SeatRef` _returnvalue (`self.OwnerCustomer`)))
      (`Customer_Seat.SetOccupied` _output_get true)
      (return true)
      (else
        (`KismetSystemLibrary.PrintString` "No Empty Seat")
        (return false)))
    (else
      (`KismetSystemLibrary.PrintString` "No ManagerClass!")
      (return false))))

(fn `GoToSeat`
  (returns (IsSeated :type Boolean))
  (bind _ownercustomer (`self.OwnerCustomer`))
  ;[1 1 1] Move to Seat
  (bind _returnvalue (`Customer_Seat.GetSeatWorldPosition` (`/Game/Characters/Customer/BP_Customer.SeatRef` _ownercustomer) (`/Game/Characters/Customer/BP_Customer.SeatNum` _ownercustomer)))
  (bind _location (.location _returnvalue))
  (`AIBlueprintHelperLibrary.SimpleMoveToLocation` self _location)
  ;[1 1 1] Range Check
  (`/Engine/EditorBlueprintResources/StandardMacros.CompareFloat` (`KismetMathLibrary.Vector_Distance` _location (`self.K2_GetActorLocation` _ownercustomer)) 100.0
    (:`>`
      (return false))
    (:`==`
      _)
    (:`<`
      _))
  (`self.K2_SetActorLocationAndRotation` (`self.OwnerCustomer`) _location (.rotation _returnvalue) false false)
  (`KismetSystemLibrary.PrintString` "IsSeated")
  (return true))

(fn `UpdateBlackboard`
  (bind _currentstate (`self.CurrentState`))
  (`BlackboardComponent.SetValueAsEnum` (`AIBlueprintHelperLibrary.GetBlackboard` null) "EnumKey" _currentstate)
  (`KismetSystemLibrary.PrintString` (`KismetStringLibrary.Concat_StrStr` "Current state " (`|GetEnumeratorNameAsString` _currentstate))))

(fn `UserConstructionScript`)